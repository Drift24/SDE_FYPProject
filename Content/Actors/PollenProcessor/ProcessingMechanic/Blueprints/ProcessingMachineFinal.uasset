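; Pollen processing machine that turns deposited flowers into launched pollen balls.
; A box overlap destroys red, blue or yellow flowers and counts them toward a required total.
; Dial and lever checks gate activation, with prompts and count shown on a text render.
; After a delay it spawns a blue pollen ball (the color shuffle is unused), applies an impulse, deducts flowers and resets both controls.
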(event `self.ReceiveBeginPlay`
  ;[1 1 1] Setting Required items for processing
  (`self.Update Text` (`self.TextRender`) (`KismetTextLibrary.Conv_IntToText` (`self.ItemCount`)))
  (set `self.Required Items` 3))

(event `Check For Flower`
  (params (Flower :type "Actor Object Reference"))
  ;[1 1 1] Checking For flowers inside machine
  (`self.K2_DestroyActor` Flower)
  (`self.UpdateCountAdd`)
  (`self.CheckForCount`)
  (if (`self.Condition Fulfilled`)
    (`self.Check for Dial`)
    (else
      (`self.Update Text` (`self.TextRender`) (`KismetTextLibrary.Conv_StringToText` (`KismetStringLibrary.Concat_StrStr` "Missing Flowers:" (`KismetStringLibrary.Conv_IntToString` (- (`self.Required Items`) (`self.ItemCount`)))))))))

(event `self.ReceiveTick`
  (params (DeltaSeconds :type "Float (single-precision)")))

(event `self.BoxCollider.OnComponentBeginOverlap`
  (params (OverlappedComponent :type "PrimitiveComponent Object Reference") (OtherActor :type "Actor Object Reference") (OtherComp :type "PrimitiveComponent Object Reference") (OtherBodyIndex :type Integer) (bFromSweep :type Boolean) (SweepResult :type "HitResult Structure (by ref)"))
  ;[1 1 1] Machine Process
  (bind _asbp_red_flower (cast `/Game/Models/MS2_Environment/Props/BP_RedFlower` OtherActor)
    (:`then`
      (`self.Check For Flower` _asbp_red_flower))
    (:`CastFailed`
      (bind _asbp_blue_flower (cast `/Game/Models/MS2_Environment/Props/BP_BlueFlower` OtherActor)
        (:`then`
          (`self.Check For Flower` _asbp_blue_flower))
        (:`CastFailed`
          (bind _asbp_yellow_flower (cast `/Game/Models/MS2_Environment/Props/BP_YellowFlower` OtherActor))
          (`self.Check For Flower` _asbp_yellow_flower))))))

(event `UpdateCountUI`
  (params (Value :type Text))
  ;[1 1 1] Update Count for items in processor
  (`self.Update Text` (`self.TextRender`) Value))

(event `SpawnPollenBall`
  ;[1 1 1] Randomize Pollen Colour
  (`KismetArrayLibrary.Array_Shuffle` (`|MakeArray` "/Game/Actors/PollenProcessor/ProcessingMechanic/Blueprints/BP_BluePollenBall.BP_BluePollenBall_C" "/Game/Actors/PollenProcessor/ProcessingMechanic/Blueprints/BP_RedPollenBall.BP_RedPollenBall_C" "/Game/Actors/PollenProcessor/ProcessingMechanic/Blueprints/BP_YellowPollenBall.BP_YellowPollenBall_C" :!type "Actor Class Reference"))
  (if (`self.Is Activated`)
    ;[1 1 1] Spawn the ball at a random location
    (`KismetSystemLibrary.Delay` 2.0)
    (`SceneComponent.K2_SetWorldRotation` (`self.Ball Spawn Pos`) (`KismetMathLibrary.MakeRotator` 0.0 (`KismetMathLibrary.RandomFloatInRange` 35.0 125.0) (`KismetMathLibrary.RandomFloatInRange` 0.0 360.0)) false false)
    (bind _returnvalue (`|SpawnActorFromClass` "/Game/Actors/PollenProcessor/ProcessingMechanic/Blueprints/BP_BluePollenBall.BP_BluePollenBall_C" (`SceneComponent.K2_GetComponentToWorld` (`self.Ball Spawn Pos`)) "Undefined" "MultiplyWithRoot" null null))
    (bind _staticmeshcomponent (`StaticMeshActor.StaticMeshComponent` _returnvalue))
    ;[1 1 1] Check if there are remaining Flowers
    (`PrimitiveComponent.AddImpulse` _staticmeshcomponent (* (`SceneComponent.GetForwardVector` _staticmeshcomponent) (0.0 2500.0 2500.0)) "None" false)
    (`self.UpdateCountSub`)
    (`self.CheckForCount`)
    (`self.UpdateCountUI` (`KismetTextLibrary.Conv_IntToText` (`self.ItemCount`)))
    (set `self.Lever Pulled` false)
    (set `self.Dial Completed` false)
    (else
      (`self.Update Text` (`self.TextRender`) (`KismetTextLibrary.Conv_StringToText` "Pull the lever")))))

(event `UpdateCountSub`
  (set `self.ItemCount` (- (`self.ItemCount`) (`self.Required Items`))))

(event `UpdateCountAdd`
  (set `self.ItemCount` (+ (`self.ItemCount`) 1)))

(event `Check for Lever`
  ;[1 1 1] Check for Lever and Dial Interactions
  (if (`self.Dial Completed`)
    (if (`self.Lever Pulled`)
      (set `self.Is Activated` true)
      (if (`self.Dial Completed`)
        ;[1 1 1] Check for Flower Count
        (if (`self.Condition Fulfilled`)
          (`self.SpawnPollenBall`)
          ;[1 1 1] Reset Interactions for next Activation
          (`self.UpdateCountUI` (`KismetTextLibrary.Conv_IntToText` (`self.ItemCount`)))
          (`self.Update Text` (`self.TextRender`) (`KismetTextLibrary.Conv_StringToText` "Processing"))
          (else
            (`self.Update Text` (`self.TextRender`) (`KismetTextLibrary.Conv_StringToText` "Not Enough Flowers"))
            (set `self.Lever Pulled` false)
            (`KismetSystemLibrary.Delay` 1.0)
            (`self.UpdateCountUI` (`KismetTextLibrary.Conv_IntToText` (`self.ItemCount`)))))
        (else
          (set `self.Lever Pulled` false)))
      (else
        (set `self.Is Activated` false)
        (if (`self.Condition Fulfilled`)
          (`self.Update Text` (`self.TextRender`) (`KismetTextLibrary.Conv_StringToText` "Pull the lever")))))
    (else
      (`self.Update Text` (`self.TextRender`) (`KismetTextLibrary.Conv_StringToText` "Turn The Dial")))))

(event `CheckForCount`
  (if (>= (`self.ItemCount`) (`self.Required Items`))
    (set `self.Condition Fulfilled` true)
    (else
      (set `self.Condition Fulfilled` false))))

(event `Update Text`
  (params (Target :type "TextRenderComponent Object Reference") (Value :type Text))
  (`TextRenderComponent.K2_SetText` Target Value))

(event `Check for Dial`
  ;[1 1 1] Check for Dial interaction
  (`self.CheckForCount`)
  (if (`self.Condition Fulfilled`)
    (if (`self.Dial Completed`)
      (`self.Check for Lever`)
      (else
        (`self.Update Text` (`self.TextRender`) (`KismetTextLibrary.Conv_StringToText` "Turn The Dial"))))
    (else
      (`TextRenderComponent.K2_SetText` (`self.TextRender`) (`KismetTextLibrary.Conv_StringToText` "Not Enough Flowers"))
      (`KismetSystemLibrary.Delay` 1.0)
      (`self.UpdateCountUI` (`KismetTextLibrary.Conv_IntToText` (`self.ItemCount`))))))

(fn `UserConstructionScript`)