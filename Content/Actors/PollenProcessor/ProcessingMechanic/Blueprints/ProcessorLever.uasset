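; VR lever actor for the Pollen Processor, operated by gripping a separate physics handle.
; Gripping the handle makes the same controller, if it has grip authority, slot-grip the VRLever after a zero-second delay that works around hand attachment.
; The lever's GripID is stored so dropping the handle also releases the lever.
; Rotating-handle events for an alternative lever method are empty stubs.
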(event `self.LeverPhysicsHandle.OnDropped`
  (params (GrippingController :type "GripMotionControllerComponent Object Reference") (GripInformation :type "BPActorGripInformation Structure (by ref)") (bWasSocketed :type Boolean))
  (bind _gripid (`self.GripID`))
  (if (> _gripid 0)
    (`GripMotionControllerComponent.DropObjectByInterface` GrippingController null _gripid (0.0 0.0 0.0) (0.0 0.0 0.0))))

(event `self.LeverRotatingHandle.OnDropped`
  (params (GrippingController :type "GripMotionControllerComponent Object Reference") (GripInformation :type "BPActorGripInformation Structure (by ref)") (bWasSocketed :type Boolean))
  ;[1 1 1] Alternative lever method
)

(event `self.LeverRotatingHandle.OnGripped`
  (params (GrippingController :type "GripMotionControllerComponent Object Reference") (GripInformation :type "BPActorGripInformation Structure (by ref)"))
  ;[1 1 1] Alternative lever method
)

(event `self.LeverPhysicsHandle.OnGripped`
  (params (GrippingController :type "GripMotionControllerComponent Object Reference") (GripInformation :type "BPActorGripInformation Structure (by ref)"))
  (bind _vrlever (`self.VRLever`))
  (if (`GripMotionControllerComponent.BP_HasGripAuthorityForObject` GrippingController _vrlever)
    (`KismetSystemLibrary.Delay` 0.0) ; This is here because the grasping hand needs a delay or it will try to attach to the second grip\nLater on I added the DontAttachHand gameplay tag and used that instead, without that re-attach this.
    (`GripMotionControllerComponent.GripObjectByInterface` GrippingController _vrlever (`SceneComponent.K2_GetComponentToWorld` _vrlever) false "None" "None" true)))

(event `self.VRLever.OnGripped`
  (params (GrippingController :type "GripMotionControllerComponent Object Reference") (GripInformation :type "BPActorGripInformation Structure (by ref)"))
  (set `self.GripID` (`.GripID` (break `BPActorGripInformation` GripInformation))))

(fn `UserConstructionScript`
  (`parent.UserConstructionScript`))