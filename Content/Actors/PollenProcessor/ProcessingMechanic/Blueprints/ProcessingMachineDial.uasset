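; Pollen processor machine actor that turns deposited flower pickups into randomly colored pollen balls once a dial is completed.
; Overlapping BP_PickupCube actors are destroyed and counted toward a threshold of required items, with status shown on a TextRender.
; CheckForDial combines that threshold with the DialCompleted flag, which this graph only resets, to trigger processing.
; After a delay, a random blue, red or yellow ball spawns at a randomized rotation and the count drops.
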(event `self.ReceiveBeginPlay`
  (`TextRenderComponent.K2_SetText` (`self.TextRender`) (`KismetTextLibrary.Conv_IntToText` (`self.ItemCount`)))
  (set `self.Required Items` 3))

(event `self.ReceiveTick`
  (params (DeltaSeconds :type "Float (single-precision)")))

(event `self.BoxCollider.OnComponentBeginOverlap`
  (params (OverlappedComponent :type "PrimitiveComponent Object Reference") (OtherActor :type "Actor Object Reference") (OtherComp :type "PrimitiveComponent Object Reference") (OtherBodyIndex :type Integer) (bFromSweep :type Boolean) (SweepResult :type "HitResult Structure (by ref)"))
  (bind _asbp_pickup_cube (cast `/Game/VRE/Grippables/Misc/Examples/BP_PickupCube` OtherActor))
  (bind _output_get (set `self.ItemCount` (+ (`self.ItemCount`) 1)))
  (`self.K2_DestroyActor` _asbp_pickup_cube)
  (bind _output_get_2 (set `self.Condition Fulfilled` (>= _output_get (`self.Required Items`))))
  (if _output_get_2
    (`self.Check for Dial`)
    (else
      (`TextRenderComponent.K2_SetText` (`self.TextRender`) (`KismetTextLibrary.Conv_StringToText` (`KismetStringLibrary.Concat_StrStr` "Missing Flowers:" (`KismetStringLibrary.Conv_IntToString` (- (`self.Required Items`) (`self.ItemCount`)))))))))

(event `UpdateCount`
  ;[1 1 1] Update Count for items in processor
  (`TextRenderComponent.K2_SetText` (`self.TextRender`) (`KismetTextLibrary.Conv_IntToText` (`self.ItemCount`))))

(event `SpawnPollenBall`
  (bind _array (`|MakeArray` "/Game/Actors/PollenProcessor/ProcessingMechanic/Blueprints/New_BP_BluePollenBall.New_BP_BluePollenBall_C" "/Game/Actors/PollenProcessor/ProcessingMechanic/Blueprints/BP_RedPollenBall.BP_RedPollenBall_C" "/Game/Actors/PollenProcessor/ProcessingMechanic/Blueprints/BP_YellowPollenBall.BP_YellowPollenBall_C" :!type "Actor Class Reference"))
  (`TextRenderComponent.K2_SetText` (`self.TextRender`) (`KismetTextLibrary.Conv_StringToText` "Processing"))
  (`KismetArrayLibrary.Array_Shuffle` _array)
  (if (`self.Is Activated`)
    (`KismetSystemLibrary.Delay` 2.0)
    (`SceneComponent.K2_SetWorldRotation` (`self.Ball Spawn Pos`) (`KismetMathLibrary.MakeRotator` 0.0 (`KismetMathLibrary.RandomFloatInRange` 35.0 125.0) (`KismetMathLibrary.RandomFloatInRange` 0.0 360.0)) false false)
    (`|SpawnActorFromClass` (`KismetArrayLibrary.Array_Random` _array) (`SceneComponent.K2_GetComponentToWorld` (`self.Ball Spawn Pos`)) "Undefined" "MultiplyWithRoot" null null)
    (set `self.ItemCount` (- (`self.ItemCount`) 3))
    (`self.UpdateCount`)
    (if (>= (`self.ItemCount`) (`self.Required Items`))
      (set `self.Condition Fulfilled` true)
      (else
        (set `self.Condition Fulfilled` false)))))

(event `Check for Dial`
  (if (`self.Dial Completed`)
    (set `self.Is Activated` true)
    (if (`self.Condition Fulfilled`)
      (`self.SpawnPollenBall`)
      (set `self.Dial Completed` false)
      (else
        (`TextRenderComponent.K2_SetText` (`self.TextRender`) (`KismetTextLibrary.Conv_StringToText` "Not Enough Flowers"))
        (set `self.Dial Completed` false)
        (`KismetSystemLibrary.Delay` 1.0)
        (`TextRenderComponent.K2_SetText` (`self.TextRender`) (`KismetTextLibrary.Conv_IntToText` (`self.ItemCount`)))))
    (else
      (set `self.Is Activated` false)
      (if (`self.Condition Fulfilled`)
        (`TextRenderComponent.K2_SetText` (`self.TextRender`) (`KismetTextLibrary.Conv_StringToText` "Turn The Dial"))))))

(fn `UserConstructionScript`)