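; ProcessorDial is a VR dial actor for the pollen processing machine that the player turns to a target count of five rotations.
; Gripping enables actor tick, which shows the rounded turn count on a text render and checks it against the target; release disables tick.
; At the target, it sets DialCompleted on its parent ProcessingMachineFinal, triggers the machine's lever check, then resets dial and flag after a delay.
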(event `self.ReceiveTick`
  (params (DeltaSeconds :type "Float (single-precision)"))
  (`self.UpdateText` :!label _label)
  (`self.CheckForActivation`))

(event `VRGripInterface.OnChildGrip`
  (params (GrippingController :type "GripMotionControllerComponent Object Reference") (GripInformation :type "BPActorGripInformation Structure (by ref)"))
  (`self.SetActorTickEnabled` true) ; The dial components tick is off
  (goto _label))

(event `CheckForActivation`
  (bind _returnvalue (`self.GetAttachParentActor`))
  (bind _output_get (set `self.IsActivated` (== (`KismetMathLibrary.Round` (/ (`VRDialComponent.CurrentDialAngle` (`self.VRDial`)) 360.0)) 5.0)))
  (if _output_get
    (bind _asprocessing_machine_final (cast `/Game/Actors/PollenProcessor/ProcessingMechanic/Blueprints/ProcessingMachineFinal` _returnvalue))
    (set `/Game/Actors/PollenProcessor/ProcessingMechanic/Blueprints/ProcessingMachineFinal.Dial Completed` true _asprocessing_machine_final)
    (`/Game/Actors/PollenProcessor/ProcessingMechanic/Blueprints/ProcessingMachineFinal.Check for Lever` _asprocessing_machine_final)
    (`KismetSystemLibrary.Delay` 7.5)
    (`self.Reset Dial`)
    (set `/Game/Actors/PollenProcessor/ProcessingMechanic/Blueprints/ProcessingMachineFinal.Dial Completed` false _asprocessing_machine_final)
    (`TextRenderComponent.K2_SetText` (`self.TextRender`) (`KismetTextLibrary.Conv_IntToText` (`KismetMathLibrary.Round` (/ (`VRDialComponent.CurrentDialAngle` (`self.VRDial`)) 360.0))))
    (else
      (bind _asprocessing_machine_final_2 (cast `/Game/Actors/PollenProcessor/ProcessingMechanic/Blueprints/ProcessingMachineFinal` _returnvalue))
      (set `/Game/Actors/PollenProcessor/ProcessingMechanic/Blueprints/ProcessingMachineFinal.Dial Completed` false _asprocessing_machine_final_2))))

(event `Reset Dial`
  (`VRDialComponent.SetDialAngle` (`self.VRDial`) 0.0 false))

(event `VRGripInterface.OnChildGripRelease`
  (params (ReleasingController :type "GripMotionControllerComponent Object Reference") (GripInformation :type "BPActorGripInformation Structure (by ref)") (bWasSocketed :type Boolean))
  (`self.SetActorTickEnabled` false))

(event `UpdateText`
  (`TextRenderComponent.K2_SetText` (`self.TextRender`) (`KismetTextLibrary.Conv_IntToText` (`KismetMathLibrary.Round` (/ (`VRDialComponent.CurrentDialAngle` (`self.VRDial`)) 360.0)))))

(fn `UserConstructionScript`)