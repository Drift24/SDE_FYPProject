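; Butterfly seed actor that turns into a randomly colored flower.
; After a fixed delay from BeginPlay, it picks a blue, red or yellow flower class, spawns it at the SeedBody's relative transform and destroys itself.
; The Sphere overlap event is empty, and a name-based ground-hit check that would trigger the same spawn is left disconnected, so only the timer drives it.
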(event `self.ReceiveBeginPlay`
  (`KismetSystemLibrary.Delay` 6.0)
  (bind _output_get (set `self.Random` (`KismetMathLibrary.RandomInteger` 3)))
  (if (== _output_get 0)
    (`|SpawnActorFromClass` "/Game/Models/MS2_Environment/Props/BP_BlueFlower.BP_BlueFlower_C" (`SceneComponent.GetRelativeTransform` (`self.SeedBody`)) "Undefined" "MultiplyWithRoot" null null)
    (`self.K2_DestroyActor` :!label _label)
    (elif (== _output_get 1)
      (`|SpawnActorFromClass` "/Game/Models/MS2_Environment/Props/BP_RedFlower.BP_RedFlower_C" (`SceneComponent.GetRelativeTransform` (`self.SeedBody`)) "Undefined" "MultiplyWithRoot" null null)
      (goto _label)
      (elif (== _output_get 2)
        (`|SpawnActorFromClass` "/Game/Models/MS2_Environment/Props/BP_YellowFlower.BP_YellowFlower_C" (`SceneComponent.GetRelativeTransform` (`self.SeedBody`)) "Undefined" "MultiplyWithRoot" null null)
        (goto _label)))))

(event `self.ReceiveTick`
  (params (DeltaSeconds :type "Float (single-precision)")))

(event `self.Sphere.OnComponentBeginOverlap`
  (params (OverlappedComponent :type "PrimitiveComponent Object Reference") (OtherActor :type "Actor Object Reference") (OtherComp :type "PrimitiveComponent Object Reference") (OtherBodyIndex :type Integer) (bFromSweep :type Boolean) (SweepResult :type "HitResult Structure (by ref)")))

(fn `UserConstructionScript`)