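; Gold butterfly seed (pollen) actor that turns into a wildflower after landing.
; A hit on the body against the actor named "Player_Area_Ground2" marks it grounded.
; Tick then lerps the body's scale toward zero and, once tiny, spawns BP_WildFlower at the body's relative transform and destroys itself.
; Colour-balancing logic for blue, red and yellow flowers is present but disabled or unused.
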(event `self.ReceiveTick`
  (params (DeltaSeconds :type "Float (single-precision)"))
  (bind _seedbody (`self.SeedBody`))
  (bind _returnvalue (`KismetMathLibrary.VLerp` (`SceneComponent.K2_GetComponentScale` _seedbody) (0.0 0.0 0.0) 0.025))
  ;[1 1 1] Minimizing pollen animation
  (if (`self.IsGrounded`)
    (`SceneComponent.SetRelativeScale3D` _seedbody _returnvalue)
    (if (< (.x _returnvalue) 0.01)
      (`self.SpawnFlower`))))

(event `self.SeedBody.OnComponentHit`
  (params (HitComponent :type "PrimitiveComponent Object Reference") (OtherActor :type "Actor Object Reference") (OtherComp :type "PrimitiveComponent Object Reference") (NormalImpulse :type "Vector Structure") (Hit :type "HitResult Structure (by ref)"))
  ;[1 1 1] Check Hit Ground
  (if (`KismetStringLibrary.EqualEqual_StrStr` (`KismetSystemLibrary.GetDisplayName` OtherActor) "Player_Area_Ground2")
    (set `self.IsGrounded` true)))

(event `SpawnFlower`
  ;[1 1 1] Spawn flowers
  (if true
    (`|SpawnActorFromClass` "/Game/Models/MS2_Environment/Props/BP_WildFlower.BP_WildFlower_C" (`SceneComponent.GetRelativeTransform` (`self.SeedBody`)) "Undefined" "MultiplyWithRoot" null null)
    (`self.K2_DestroyActor`)))

(fn `UserConstructionScript`)