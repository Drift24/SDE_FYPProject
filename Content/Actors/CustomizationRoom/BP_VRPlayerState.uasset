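; VR player state Blueprint that shares the headset's device position and flags when the player is too close to others.
; On BeginPlay, the local controller starts a one-second loop sending device position to a server event that stores it.
; A second one-second loop watches IsTooCloseToOthers, which is set outside these graphs, toggling IsWidgetVisible and printing a warning.
; The HUD widget show and hide calls are disconnected.
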(event `self.ReceiveBeginPlay`
  (`self.UpdateDevPos`)
  (`self.NearOtherDevices`))

(event `NearOtherDevices`
  (if (`Controller.IsLocalController` (`self.GetPlayerController`))
    (bind _astemplate_vr_player_controller (cast `/Game/VRE/Core/Template_VR_Player_Controller` (`self.GetPlayerController`)))
    (if (and (`self.IsTooCloseToOthers`) (not (`self.IsWidgetVisible`))) :!label _label
      (set `self.IsWidgetVisible` true)
      (`KismetSystemLibrary.PrintString` "Too near to others" true true (struct :`R` 1.0 :`A` 1.0) 1.0)
      (elif (and (not (`self.IsTooCloseToOthers`)) (`self.IsWidgetVisible`))
        (set `self.IsWidgetVisible` false)))
    (`KismetSystemLibrary.Delay` 1.0)
    (goto _label)))

(event `UpdateDevPos`
  ;[1 1 1] Update device position to server
  (if (`Controller.IsLocalController` (`self.GetPlayerController`)) :!label _label_2
    (`self.SERVER_UpdateDevicePos` (`.DevicePosition` (`HeadMountedDisplayFunctionLibrary.GetOrientationAndPosition`)))
    (`KismetSystemLibrary.Delay` 1.0)
    (goto _label_2)))

(event `SERVER_UpdateDevicePos`
  (params (DevicePos :type "Vector Structure"))
  (set `self.DevicePos` DevicePos))

(fn `UserConstructionScript`)