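; Butterfly actor that flies toward a Target actor using steering behaviours and periodically drops scaled-down butterfly seed actors.
; Each Tick sums a seek vector with an obstacle avoidance vector, derived from a sphere trace along the current velocity.
; The clamped velocity is smoothed by SteeringTime, then moves the actor and turns it to face its direction of travel.
; A Delay loop from BeginPlay drives seed spawning; an older basic-movement chain is left unconnected.
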(event `self.ReceiveBeginPlay`
  ;[1 1 1] Periodically Spawn Butterfly Seeds
  (`KismetSystemLibrary.Delay` 10.0 :!label _label)
  (`self.SpawnSeeds`)
  (goto _label))

(event `self.ReceiveTick`
  (params (DeltaSeconds :type "Float (single-precision)"))
  (bind _returnvalue (`self.K2_GetActorLocation`))
  (bind _max_velocity (`self.Max Velocity`))
  (bind _max_velocity_2 (`self.Max Velocity`))
  (bind _steeringtime (`self.SteeringTime`))
  (bind _max_velocity_3 (`self.Max Velocity`))
  ;[1 1 1] Seek
  ;;[1 1 1] Clamp to maximum velocity
  (bind _output_get (set `self.Desired Velocity` (`KismetMathLibrary.ClampVectorSize` (`KismetMathLibrary.Conv_RotatorToVector` (`KismetMathLibrary.FindLookAtRotation` (`self.K2_GetActorLocation`) (`self.K2_GetActorLocation` (`self.Target`)))) (* _max_velocity_3 -1.0) _max_velocity_3)))
  (set `self.SteeringVector` (* (- _output_get (`self.Current Velocity`)) (`self.SeekWeight`)))
  ;[1 1 1] Obstacle Avoidance
  (bind (_outhit _returnvalue_2) (`KismetSystemLibrary.SphereTraceSingleForObjects` _returnvalue (+ (* (`KismetMathLibrary.Normal` (`self.Current Velocity`)) (`self.ObstacleCheckDist`)) _returnvalue) (`self.ObstacleCheckRadius`) (`self.ObstacleCheckTypes`)))
  (if _returnvalue_2
    (set `self.SteeringVector` (+ (* (- (`KismetMathLibrary.ClampVectorSize` (- (+ (* (`KismetMathLibrary.Cross_VectorVector` (`SceneComponent.GetUpVector` (`self.Player_Area_BlueButterfly_Fly`)) (`self.Current Velocity`)) (`self.AvoidDistance`)) (`.ImpactPoint` (`GameplayStatics.BreakHitResult` _outhit))) (`self.K2_GetActorLocation`)) (* _max_velocity_2 -1.0) _max_velocity_2) (`self.Current Velocity`)) (`self.ObstacleAvoidanceWeight`)) (`self.SteeringVector`))))
  ;[1 1 1] Move Entity
  (bind _output_get_2 (set `self.ExpectedEndPosition` (+ (`self.K2_GetActorLocation`) (`KismetMathLibrary.ClampVectorSize` (+ (`self.Current Velocity`) (`self.SteeringVector`)) (* _max_velocity -1.0) _max_velocity))))
  ;;[1 1 1] Attempt To Simulate Smooth Damping
  (if (<= _steeringtime 1.0)
    (bind _returnvalue_3 (- _output_get_2 (`self.K2_GetActorLocation`)))
    (set `self.Current Velocity` _returnvalue_3)
    (else
      (set `self.Current Velocity` (+ (/ (- _returnvalue_3 (`self.Current Velocity`)) _steeringtime) (`self.Current Velocity`)))))
  (`self.K2_SetActorLocation` (+ (`self.Current Velocity`) (`self.K2_GetActorLocation`)))
  ;[1 1 1] Rotate Object To Move Direction
  (`self.K2_SetActorRotation` (`KismetMathLibrary.FindLookAtRotation` (`KismetMathLibrary.Vector_Zero`) (`self.Current Velocity`))))

(event `SpawnSeeds`
  ;[1 1 1] Spawn Seed
  (bind _returnvalue (`|SpawnActorFromClass` "/Game/Actors/NewButterfly/Seed/bp_butterfly_seed.bp_butterfly_seed_C" (`self.GetTransform`) "Undefined" "MultiplyWithRoot" null null))
  (`SceneComponent.SetWorldScale3D` (`Actor.RootComponent` _returnvalue) (0.05 0.05 0.05)))

(fn `UserConstructionScript`)