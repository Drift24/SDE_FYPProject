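; Butterfly seed actor that turns into a randomly chosen flower when it hits the ground, or destroys itself after a timed lifespan.
; Sphere overlap prints the other actor's name and detects ground by matching one hard-coded StaticMeshActor name.
; A random pick spawns a blue, red or yellow flower at SeedBody's relative transform, sets its scale (blue gets a larger value), then destroys the seed.
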(event `self.ReceiveBeginPlay`
  (`KismetSystemLibrary.Delay` 15.0)
  (`self.K2_DestroyActor`))

(event `self.Sphere.OnComponentBeginOverlap`
  (params (OverlappedComponent :type "PrimitiveComponent Object Reference") (OtherActor :type "Actor Object Reference") (OtherComp :type "PrimitiveComponent Object Reference") (OtherBodyIndex :type Integer) (bFromSweep :type Boolean) (SweepResult :type "HitResult Structure (by ref)"))
  (bind _returnvalue (`KismetSystemLibrary.GetObjectName` OtherActor))
  ;[1 1 1] Check Hit Ground
  (`KismetSystemLibrary.PrintString` _returnvalue)
  (if (`KismetStringLibrary.EqualEqual_StrStr` _returnvalue "StaticMeshActor_99")
    (bind _output_get (set `self.Random` (`KismetMathLibrary.RandomInteger` 3)))
    (if (== _output_get 0)
      (bind _returnvalue_2 (`|SpawnActorFromClass` "/Game/MS2_Environment/Props/BP_BlueFlower.BP_BlueFlower_C" (`SceneComponent.GetRelativeTransform` (`self.SeedBody`)) "Undefined" "MultiplyWithRoot" null null))
      (`SceneComponent.SetWorldScale3D` (`Actor.RootComponent` _returnvalue_2) (10.0 10.0 10.0))
      (`self.K2_DestroyActor` :!label _label)
      (elif (== _output_get 1)
        (bind _returnvalue_3 (`|SpawnActorFromClass` "/Game/MS2_Environment/Props/BP_RedFlower.BP_RedFlower_C" (`SceneComponent.GetRelativeTransform` (`self.SeedBody`)) "Undefined" "MultiplyWithRoot" null null))
        (`SceneComponent.SetWorldScale3D` (`Actor.RootComponent` _returnvalue_3) (1.0 1.0 1.0))
        (goto _label)
        (elif (== _output_get 2)
          (bind _returnvalue_4 (`|SpawnActorFromClass` "/Game/MS2_Environment/Props/BP_YellowFlower.BP_YellowFlower_C" (`SceneComponent.GetRelativeTransform` (`self.SeedBody`)) "Undefined" "MultiplyWithRoot" null null))
          (`SceneComponent.SetWorldScale3D` (`Actor.RootComponent` _returnvalue_4) (1.0 1.0 1.0))
          (goto _label))))))

(fn `UserConstructionScript`)