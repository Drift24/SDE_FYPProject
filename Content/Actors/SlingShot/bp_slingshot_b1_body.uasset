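; Slingshot body actor that aims and fires a projectile when its child-actor holder is gripped, pulled back and released.
; A 0.1-second looping timer polls the holder's grip state, yawing the body along the pull while gripped.
; Beyond a minimum pull, it spawns trajectory marker actors along a predicted path.
; Release applies force scaled by pull distance to a spawned projectile; prediction uses that same vector as launch velocity.
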(event `self.ReceiveBeginPlay`
  (`KismetSystemLibrary.K2_SetTimerDelegate` (delegate `CheckShootUpdate`) 0.1 true true))

(event `CheckShootUpdate`
  (`self.CheckShoot`))

(event `self.ReceiveTick`
  (params (DeltaSeconds :type "Float (single-precision)")))

(event `CheckShoot`
  (bind _asbp_slingshot_b_1_holder (cast `/Game/Actors/SlingShot/bp_slingshot_b1_holder` (`ChildActorComponent.ChildActor` (`self.Holder`))))
  (bind _gripped (`/Game/Actors/SlingShot/bp_slingshot_b1_holder.Gripped` _asbp_slingshot_b_1_holder))
  ;[1 1 1] Check For Change in Status of Grip
  (if (!= _gripped (`self.GrippingHolder`))
    ;[1 1 1] Check To Shoot
    (if _gripped
      (set `self.GrippingHolder` _gripped)
      (else
        (bind _returnvalue (`SceneComponent.K2_GetComponentLocation` (`StaticMeshActor.StaticMeshComponent` _asbp_slingshot_b_1_holder)))
        (bind _returnvalue_2 (`KismetMathLibrary.Vector_Distance` (`SceneComponent.K2_GetComponentLocation` (`self.StartPos`)) _returnvalue))
        (bind _returnvalue_3 (>= _returnvalue_2 (`self.MinDistToShoot`)))
        ;[1 1 1] Shoot Projectile
        (if _returnvalue_3
          (bind _returnvalue_4 (`|SpawnActorFromClass` "/Game/VRE/Grippables/Weapons/Guns/FirstPersonProjectile.FirstPersonProjectile_C" (`SceneComponent.K2_GetComponentToWorld` (`self.StartPos`)) "Undefined" "MultiplyWithRoot" null null))
          (bind _rootcomponent (`Actor.RootComponent` _returnvalue_4))
          (`SceneComponent.K2_SetWorldLocation` _rootcomponent (`SceneComponent.K2_GetComponentLocation` (`self.FirePosition`)) false false)
          (`SceneComponent.SetWorldScale3D` _rootcomponent (1.0 1.0 1.0))
          (bind _returnvalue_5 (* (* (`KismetMathLibrary.GetDirectionUnitVector` _returnvalue (`SceneComponent.K2_GetComponentLocation` (`self.StartPos`))) _returnvalue_2) (`self.Force Scaler`)))
          (`PrimitiveComponent.AddForce` (`/Game/VRE/Grippables/Weapons/Guns/FirstPersonProjectile.CollisionComponent` _returnvalue_4) _returnvalue_5 "None" false))
        (set `self.GrippingHolder` _gripped)))
    (else
      ;[1 1 1] Rotate Slingshot
      (if _gripped
        (`self.K2_SetActorRotation` (`KismetMathLibrary.MakeRotator` 0.0 0.0 (.yaw (`KismetMathLibrary.FindLookAtRotation` (`SceneComponent.K2_GetComponentLocation` (`StaticMeshActor.StaticMeshComponent` _asbp_slingshot_b_1_holder)) (`SceneComponent.K2_GetComponentLocation` (`self.StartPos`))))))
        ;[1 1 1] Projectile Prediction
        (if _returnvalue_3
          (bind _predictresult (`GameplayStatics.Blueprint_PredictProjectilePath_Advanced` (make `PredictProjectilePathParams` (`SceneComponent.K2_GetComponentLocation` (`self.FirePosition`)) _returnvalue_5 false 0.0 1.0 true "ECC_WorldStatic" _ _ 100.0)))
          (for _array_element (break `PredictProjectilePathResult` _predictresult)
            (`|SpawnActorFromClass` "/Game/Actors/SlingShot/bp_trajectory_predictor.bp_trajectory_predictor_C" (`KismetMathLibrary.MakeTransform` (break `PredictProjectilePathPointData` _array_element)) "Undefined" "MultiplyWithRoot" null null)))))))

(fn `UserConstructionScript`)