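; A placeholder cannon actor, kept under the SlingShot TempCannon folder, that automatically fires projectiles on a repeating timer.
; A looping timer set on BeginPlay calls Shoot, which spawns a FirstPersonProjectile at the cannon's transform.
; Shoot then moves it along the forward vector plus a fixed world-space Y offset and adds forward force to its collision component.
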(event `self.ReceiveBeginPlay`
  (`KismetSystemLibrary.K2_SetTimer` null "Shoot" 0.5 true))

(event `Shoot`
  (bind _returnvalue (`|SpawnActorFromClass` "/Game/VRE/Grippables/Weapons/Guns/FirstPersonProjectile.FirstPersonProjectile_C" (`self.GetTransform`) "Undefined" "MultiplyWithRoot" null null))
  (`self.K2_SetActorLocation` _returnvalue (+ (`self.K2_GetActorLocation`) (+ (* (`self.GetActorForwardVector`) 50.0) (0.0 100.0 0.0))) false false)
  (`PrimitiveComponent.AddForce` (`/Game/VRE/Grippables/Weapons/Guns/FirstPersonProjectile.CollisionComponent` _returnvalue) (* (`self.GetActorForwardVector`) 50.0) "None" false))

(fn `UserConstructionScript`)