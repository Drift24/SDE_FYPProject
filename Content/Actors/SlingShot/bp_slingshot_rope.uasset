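; Slingshot rope actor that visually stretches between two bind targets, LeftBindTarget and RightBindTarget.
; Each Tick it moves its root to their midpoint, aligns it along the direction between them and scales X by their distance.
; The Stretch event is an empty stub, and its looping timer and a debug print are left unconnected.
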(event `self.ReceiveBeginPlay`)

(event `StretchUpdate`
  (`self.Stretch`))

(event `Stretch`)

(event `self.ReceiveTick`
  (params (DeltaSeconds :type "Float (single-precision)"))
  (bind _returnvalue (`self.K2_GetActorLocation` (`self.LeftBindTarget`)))
  ;[1 1 1] Scale Rope
  (`SceneComponent.SetWorldScale3D` (`self.DefaultSceneRoot`) (`KismetMathLibrary.MakeVector` (/ (`KismetMathLibrary.Vector_Distance` (`self.K2_GetActorLocation` (`self.LeftBindTarget`)) (`self.K2_GetActorLocation` (`self.RightBindTarget`))) 60.0) 1.0 1.0))
  ;[1 1 1] Location
  (`SceneComponent.K2_SetWorldLocation` (`self.DefaultSceneRoot`) (- _returnvalue (/ (- _returnvalue (`self.K2_GetActorLocation` (`self.RightBindTarget`))) 2.0)) false false)
  ;[1 1 1] Rotation
  (`SceneComponent.K2_SetWorldRotation` (`self.DefaultSceneRoot`) (`KismetMathLibrary.Quat_Rotator` (`KismetMathLibrary.Conv_VectorToQuaternion` (`KismetMathLibrary.Normal` (- (`self.K2_GetActorLocation` (`self.LeftBindTarget`)) (`self.K2_GetActorLocation` (`self.RightBindTarget`))) 1.0))) false false))

(fn `UserConstructionScript`)