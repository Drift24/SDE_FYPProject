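; Slingshot body actor that fires pollen balls, reloaded one at a time by overlapping a blue pollen ball with its collider.
; BeginPlay binds both rope child actors to the frame and pouch holder, then starts a looping timer that polls the holder's grip.
; While gripped and pulled far enough, it yaws along the pull and draws a predicted arc with short-lived marker actors.
; Release spawns a projectile pushed by pull-scaled force, carrying the loaded damage.
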(event `self.ReceiveTick`
  (params (DeltaSeconds :type "Float (single-precision)")))

(event `CheckShoot`
  (bind _asbp_slingshot_b_1_holder (cast `/Game/Actors/SlingShot/bp_slingshot_b1_holder` (`ChildActorComponent.ChildActor` (`self.Holder`))))
  (bind _gripped (`/Game/Actors/SlingShot/bp_slingshot_b1_holder.Gripped` _asbp_slingshot_b_1_holder))
  ;[1 1 1] Check For Change in Status of Grip
  (if (!= _gripped (`self.GrippingHolder`))
    ;[1 1 1] Check To Shoot
    (if _gripped
      (set `self.GrippingHolder` _gripped)
      (else
        (bind _returnvalue (`SceneComponent.K2_GetComponentLocation` (`StaticMeshActor.StaticMeshComponent` _asbp_slingshot_b_1_holder)))
        (bind _returnvalue_2 (`KismetMathLibrary.Vector_Distance` (`SceneComponent.K2_GetComponentLocation` (`self.StartPos`)) _returnvalue))
        (bind _returnvalue_3 (>= _returnvalue_2 (`self.MinDistToShoot`)))
        ;[1 1 1] Shoot Projectile
        (if _returnvalue_3
          (`KismetSystemLibrary.PrintText` "Can Shoot")
          ;;[1 1 1] Check of got projectiles in ammo
          (if (> (`self.bullet`) 0)
            (`KismetSystemLibrary.PrintText` "Have Ammo")
            (bind _returnvalue_4 (`|SpawnActorFromClass` "/Game/Actors/SlingShot/BP_ProjPollenBall.BP_ProjPollenBall_C" (`SceneComponent.K2_GetComponentToWorld` (`self.StartPos`)) "Undefined" "MultiplyWithRoot" null null))
            (set `/Game/Actors/SlingShot/BP_ProjPollenBall.ProjDamage` (`self.DamageForPollen`) _returnvalue_4)
            (bind _rootcomponent (`Actor.RootComponent` _returnvalue_4))
            (`SceneComponent.K2_SetWorldLocation` _rootcomponent (`SceneComponent.K2_GetComponentLocation` (`self.FirePosition`)) false false)
            (`SceneComponent.SetWorldScale3D` _rootcomponent (0.2 0.2 0.2))
            (bind _returnvalue_5 (* (* (`KismetMathLibrary.GetForwardVector` (`KismetMathLibrary.FindLookAtRotation` _returnvalue (`SceneComponent.K2_GetComponentLocation` (`self.StartPos`)))) _returnvalue_2) (`self.Force Scaler`)))
            (bind (_returnvalue_x _returnvalue_y _returnvalue_z) (`KismetMathLibrary.BreakVector` (+ _returnvalue_5 (0.0 0.0 0.0))))
            (`PrimitiveComponent.AddForce` (`StaticMeshActor.StaticMeshComponent` _returnvalue_4) (`KismetMathLibrary.MakeVector` (* _returnvalue_x 120.0) (* _returnvalue_y 120.0) (* _returnvalue_z 150.0)) "None" false)
            (set `self.bullet` 0)
            (`/Game/Actors/SlingShot/bp_slingshot_b1_holder.DeactivateAmmunition` _asbp_slingshot_b_1_holder)))
        (set `self.GrippingHolder` _gripped)))
    (else
      ;[1 1 1] Rotate Slingshot
      (if _gripped
        (if _returnvalue_3
          (`self.K2_SetActorRotation` (`KismetMathLibrary.MakeRotator` 0.0 0.0 (.yaw (`KismetMathLibrary.FindLookAtRotation` (`SceneComponent.K2_GetComponentLocation` (`StaticMeshActor.StaticMeshComponent` _asbp_slingshot_b_1_holder)) (`SceneComponent.K2_GetComponentLocation` (`self.StartPos`))))))
          ;[1 1 1] Projectile Prediction
          (bind _predictresult (`GameplayStatics.Blueprint_PredictProjectilePath_Advanced` (make `PredictProjectilePathParams` (`SceneComponent.K2_GetComponentLocation` (`self.FirePosition`)) _returnvalue_5 false 0.0 1.0 true "ECC_WorldStatic" _ _ 25.0)))
          (for _array_element (break `PredictProjectilePathResult` _predictresult)
            (bind _returnvalue_6 (`|SpawnActorFromClass` "/Game/Actors/SlingShot/bp_trajectory_predictor.bp_trajectory_predictor_C" (`KismetMathLibrary.MakeTransform` (break `PredictProjectilePathPointData` _array_element)) "Undefined" "MultiplyWithRoot" null null))
            (`self.SetLifeSpan` _returnvalue_6 0.01)))))))

(event `self.ReceiveBeginPlay`
  (`KismetSystemLibrary.K2_SetTimerDelegate` (delegate `CheckShootUpdate`) 0.01 true true)
  ;[1 1 1] Left Rope
  (bind _asbp_slingshot_rope (cast `/Game/Actors/SlingShot/bp_slingshot_rope` (`ChildActorComponent.ChildActor` (`self.rope_left`))))
  (bind _asbp_slingshot_ropebind (cast `/Game/Actors/SlingShot/bp_slingshot_ropebind` (`ChildActorComponent.ChildActor` (`self.LeftBind_Left`))))
  (set `/Game/Actors/SlingShot/bp_slingshot_rope.LeftBindTarget` _asbp_slingshot_ropebind _asbp_slingshot_rope)
  (bind _asbp_slingshot_b_1_holder (cast `/Game/Actors/SlingShot/bp_slingshot_b1_holder` (`ChildActorComponent.ChildActor` (`self.Holder`))))
  (set `/Game/Actors/SlingShot/bp_slingshot_rope.RightBindTarget` (`/Game/Actors/SlingShot/bp_slingshot_b1_holder.LeftBindVar` _asbp_slingshot_b_1_holder) _asbp_slingshot_rope)
  ;[1 1 1] Right Rope
  (bind _asbp_slingshot_rope_2 (cast `/Game/Actors/SlingShot/bp_slingshot_rope` (`ChildActorComponent.ChildActor` (`self.Rope Right`))))
  (bind _asbp_slingshot_ropebind_2 (cast `/Game/Actors/SlingShot/bp_slingshot_ropebind` (`ChildActorComponent.ChildActor` (`self.RightBind_Right`))))
  (set `/Game/Actors/SlingShot/bp_slingshot_rope.RightBindTarget` _asbp_slingshot_ropebind_2 _asbp_slingshot_rope_2)
  (bind _asbp_slingshot_b_1_holder_2 (cast `/Game/Actors/SlingShot/bp_slingshot_b1_holder` (`ChildActorComponent.ChildActor` (`self.Holder`))))
  (set `/Game/Actors/SlingShot/bp_slingshot_rope.LeftBindTarget` (`/Game/Actors/SlingShot/bp_slingshot_b1_holder.RightBindVar` _asbp_slingshot_b_1_holder_2) _asbp_slingshot_rope_2))

(event `CheckShootUpdate`
  (`self.CheckShoot`))

(event `self.Reload Collider.OnComponentBeginOverlap`
  (params (OverlappedComponent :type "PrimitiveComponent Object Reference") (OtherActor :type "Actor Object Reference") (OtherComp :type "PrimitiveComponent Object Reference") (OtherBodyIndex :type Integer) (bFromSweep :type Boolean) (SweepResult :type "HitResult Structure (by ref)"))
  (bind _asbp_blue_pollen_ball (cast `/Game/Actors/PollenProcessor/ProcessingMechanic/Blueprints/New_BP_BluePollenBall` OtherActor))
  (`self.PollenHAndle` _asbp_blue_pollen_ball))

(event `PollenHAndle`
  (params (Pollen :type "/Game/Actors/PollenProcessor/ProcessingMechanic/Blueprints/New_BP_BluePollenBall Object Reference"))
  ;[1 1 1] Check hit max bullet count
  (if (not (> (`self.bullet`) 0))
    (set `self.DamageForPollen` (`/Game/Actors/PollenProcessor/ProcessingMechanic/Blueprints/New_BP_BluePollenBall.Damage` Pollen))
    (`self.K2_DestroyActor` Pollen)
    (set `self.bullet` 1)
    (bind _asbp_slingshot_b_1_holder (cast `/Game/Actors/SlingShot/bp_slingshot_b1_holder` (`ChildActorComponent.ChildActor` (`self.Holder`))))
    (`/Game/Actors/SlingShot/bp_slingshot_b1_holder.ActivateAmmunition` _asbp_slingshot_b_1_holder)))

(fn `OnRep_MinDistToShoot`)

(fn `UserConstructionScript`)