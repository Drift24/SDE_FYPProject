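; Corruption target actor that pollen ball projectiles damage and destroy.
; On the authority, an overlap of its box by a pollen ball subtracts the projectile's damage from its lives and destroys the projectile.
; Remaining lives update a health bar widget, and at zero the target destroys itself.
; On destruction it reports itself to the FireSpreadingManager through FireDestroyed.
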(event `self.ReceiveBeginPlay`
  (bind _output_get (set `self.Lives` (+ 1 1)))
  (set `self.MaxLives` _output_get)
  (bind _aswbp_corruption_health (cast `/Game/Actors/CorruptionTargets/wbp_corruption_health` (`WidgetComponent.GetWidget` (`self.wbp_health`))))
  (set `self.wbp_corruption_health` _aswbp_corruption_health))

(event `self.Box.OnComponentBeginOverlap`
  (params (OverlappedComponent :type "PrimitiveComponent Object Reference") (OtherActor :type "Actor Object Reference") (OtherComp :type "PrimitiveComponent Object Reference") (OtherBodyIndex :type Integer) (bFromSweep :type Boolean) (SweepResult :type "HitResult Structure (by ref)"))
  (`/Engine/EditorBlueprintResources/ActorMacros.Switch Has Authority`
    (:`Authority`
      (if (== (`GameplayStatics.GetObjectClass` OtherActor) "/Game/Actors/SlingShot/BP_ProjPollenBall.BP_ProjPollenBall_C")
        (`self.TargetHit` OtherActor)))))

(event `self.ReceiveDestroyed`
  (bind _returnvalue (`GameplayStatics.GetActorOfClass` "/Game/Actors/CorruptionTargets/FireSpreadingManager.FireSpreadingManager_C"))
  (`/Game/Actors/CorruptionTargets/FireSpreadingManager.FireDestroyed` _returnvalue self))

(event `TargetHit`
  (params (Projectile :type "Actor Object Reference"))
  (bind _asbp_proj_pollen_ball (cast `/Game/Actors/SlingShot/BP_ProjPollenBall` Projectile)
    (:`then`
      (bind _output_get (set `self.Lives` (- (`self.Lives`) (`/Game/Actors/SlingShot/BP_ProjPollenBall.ProjDamage` _asbp_proj_pollen_ball))))
      (`self.K2_DestroyActor` Projectile)
      (if (<= _output_get 0)
        (`self.K2_DestroyActor`)
        (else
          (`/Game/Actors/CorruptionTargets/wbp_corruption_health.AlterHealthBar` (`self.wbp_corruption_health`) (/ _output_get (`self.MaxLives`))))))
    (:`CastFailed`
      (`KismetSystemLibrary.PrintString` "Cannot get pollen component" true true (struct :`R` 1.0 :`A` 1.0)))))

(fn `UserConstructionScript`)