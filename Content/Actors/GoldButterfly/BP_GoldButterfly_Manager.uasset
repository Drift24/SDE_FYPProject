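; BP_GoldButterfly_Manager is an actor that keeps spawning gold butterflies while fewer than two exist in the level.
; On BeginPlay it caches every BP_GoldButterFly_Spawn actor, then runs an endless delayed loop that counts live BP_GoldButterfly actors.
; When short, it spawns one at a randomly indexed spawn point's transform; the random range includes the array length, so the index can fall out of bounds.
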(event `self.ReceiveBeginPlay`
  (bind _outactors (`GameplayStatics.GetAllActorsOfClass` "/Game/Actors/GoldButterfly/BP_GoldButterFly_Spawn.BP_GoldButterFly_Spawn_C"))
  (set `self.SpawnLocations` _outactors)
  (`KismetSystemLibrary.Delay` 15.0 :!label _label)
  (bind _outactors_2 (`GameplayStatics.GetAllActorsOfClass` "/Game/Actors/GoldButterfly/BP_GoldButterfly.BP_GoldButterfly_C"))
  (if (< (`KismetArrayLibrary.Array_Length` _outactors_2) 2)
    ;[1 1 1] Handle Spawn Butter fly
    (`|SpawnActorFromClass` "/Game/Actors/GoldButterfly/BP_GoldButterfly.BP_GoldButterfly_C" (`self.GetTransform` (`|GetArrayItem` (`self.SpawnLocations`) (`KismetMathLibrary.RandomIntegerInRange` 0 (`KismetArrayLibrary.Array_Length` (`self.SpawnLocations`))))) "Undefined" "MultiplyWithRoot" null null)
    (goto _label)
    (else
      (goto _label))))

(fn `UserConstructionScript`)