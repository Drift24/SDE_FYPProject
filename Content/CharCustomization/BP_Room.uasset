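; BP_Room is an actor in the character customization folder that hosts a customization widget on its Widget component.
; On BeginPlay it assigns CustomizationWidget to the component, then logs whether the user widget object is valid, along with widget names.
; An unconnected debug branch that casts to WBP_CustomizationSelect and logs its CanDestroy flag never runs.
; Tick, overlap and construction logic are empty.
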(event `self.ReceiveBeginPlay`
  (`WidgetComponent.SetWidget` (`self.Widget`) (`self.Customization Widget`))
  (if (`KismetSystemLibrary.IsValid` (`WidgetComponent.GetUserWidgetObject` (`self.Widget`)))
    (`KismetSystemLibrary.LogString` (`KismetSystemLibrary.GetDisplayName` (`WidgetComponent.GetUserWidgetObject` (`self.Widget`))))
    (`KismetSystemLibrary.LogString` (`KismetSystemLibrary.GetDisplayName` (`WidgetComponent.GetWidget` (`self.Widget`))))
    (else
      (`KismetSystemLibrary.LogString` (`KismetSystemLibrary.GetDisplayName` (`WidgetComponent.GetWidget` (`self.Widget`))))
      (`KismetSystemLibrary.LogString` "Isn't Valid"))))

(event `self.ReceiveTick`
  (params (DeltaSeconds :type "Float (single-precision)")))

(fn `UserConstructionScript`)