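; ProcessorDial is a grippable dial for the processing mechanic that displays its angle as text.
; Gripping enables actor tick, which writes the dial component's clamped yaw to the text render with two decimals; release disables it.
; On release, if the slide indicator and angle snap are set, yaw is set to the roll snapped to the angle increment and the text refreshes.
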(event `self.ReceiveTick`
  (params (DeltaSeconds :type "Float (single-precision)"))
  (bind (_relativerotation_roll _relativerotation_pitch _relativerotation_yaw) (`KismetMathLibrary.BreakRotator` (`SceneComponent.RelativeRotation` (`self.DialComponent`))))
  (`TextRenderComponent.K2_SetText` (`self.TextRender`) (`KismetTextLibrary.Conv_DoubleToText` (`KismetMathLibrary.ClampAxis` _relativerotation_yaw) "HalfToEven" false true 1 324 2 2)))

(event `VRGripInterface.OnChildGrip`
  (params (GrippingController :type "GripMotionControllerComponent Object Reference") (GripInformation :type "BPActorGripInformation Structure (by ref)"))
  (`self.SetActorTickEnabled` true) ; The dial components tick is off
)

(event `VRGripInterface.OnChildGripRelease`
  (params (ReleasingController :type "GripMotionControllerComponent Object Reference") (GripInformation :type "BPActorGripInformation Structure (by ref)") (bWasSocketed :type Boolean))
  (bind _dialcomponent (`self.DialComponent`))
  (bind (_relativerotation_roll _relativerotation_pitch) (`KismetMathLibrary.BreakRotator` (`SceneComponent.RelativeRotation` _dialcomponent)))
  (bind (_relativerotation_roll_2 _relativerotation_pitch_2 _relativerotation_yaw) (`KismetMathLibrary.BreakRotator` (`SceneComponent.RelativeRotation` _dialcomponent)))
  ;[1 1 1] Snap To Increment On Release if it is a slider dial
  (`self.SetActorTickEnabled` false)
  (if (and (`self.bSlideIndictor`) (`self.DialAngleSnap`))
    (`SceneComponent.K2_SetRelativeRotation` _dialcomponent (`KismetMathLibrary.MakeRotator` _relativerotation_roll _relativerotation_pitch (`KismetMathLibrary.GridSnap_Float` _relativerotation_roll (`self.SnapAngleIncrement`))) false false)
    (`TextRenderComponent.K2_SetText` (`self.TextRender`) (`KismetTextLibrary.Conv_DoubleToText` (`KismetMathLibrary.ClampAxis` _relativerotation_yaw) "HalfToEven" false true 1 324 2 2))))

(fn `UserConstructionScript`)