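; Processing machine that collects flower pickups and turns every three into a randomly colored pollen ball.
; Overlapping pickup cubes are destroyed and counted, with a text render showing the count, missing flowers or status.
; At three items it calls SpawnPollenBall if LeverPulled is set, otherwise it prompts for the lever and still calls it in a loop after a delay.
; SpawnPollenBall waits briefly, spawns a blue, red or yellow ball at BallSpawnPos, then deducts three items.
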(event `self.ReceiveBeginPlay`
  (`TextRenderComponent.K2_SetText` (`self.TextRender`) (`KismetTextLibrary.Conv_IntToText` (`self.ItemCount`))))

(event `self.ReceiveTick`
  (params (DeltaSeconds :type "Float (single-precision)")))

(event `self.BoxCollider.OnComponentBeginOverlap`
  (params (OverlappedComponent :type "PrimitiveComponent Object Reference") (OtherActor :type "Actor Object Reference") (OtherComp :type "PrimitiveComponent Object Reference") (OtherBodyIndex :type Integer) (bFromSweep :type Boolean) (SweepResult :type "HitResult Structure (by ref)"))
  (bind _asbp_pickup_cube (cast `/Game/VRE/Grippables/Misc/Examples/BP_PickupCube` OtherActor))
  (bind _output_get (set `self.ItemCount` (+ (`self.ItemCount`) 1)))
  (`self.K2_DestroyActor` _asbp_pickup_cube)
  (bind _output_get_2 (set `self.Condition Fulfilled` (== _output_get 3)))
  (if _output_get_2
    (if (`self.Lever Pulled`)
      (`self.SpawnPollenBall`)
      (else
        (`TextRenderComponent.K2_SetText` (`self.TextRender`) (`KismetTextLibrary.Conv_StringToText` "Pull the lever"))
        (`KismetSystemLibrary.Delay` 5.0)
        (for _ (range 6)
          (`self.SpawnPollenBall`))))
    (else
      (`TextRenderComponent.K2_SetText` (`self.TextRender`) (`KismetTextLibrary.Conv_StringToText` (`KismetStringLibrary.Concat_StrStr` "Missing Flowers:" (`KismetStringLibrary.Conv_IntToString` (- 3 (`self.ItemCount`)))))))))

(event `UpdateCount`
  ;[1 1 1] Update Count for items in processor
  (`TextRenderComponent.K2_SetText` (`self.TextRender`) (`KismetTextLibrary.Conv_IntToText` (`self.ItemCount`))))

(event `SpawnPollenBall`
  (bind _array (`|MakeArray` "/Game/ProcessingMechanic/Blueprints/BP_BluePollenBall.BP_BluePollenBall_C" "/Game/ProcessingMechanic/Blueprints/BP_RedPollenBall.BP_RedPollenBall_C" "/Game/ProcessingMechanic/Blueprints/BP_YellowPollenBall.BP_YellowPollenBall_C" :!type "Actor Class Reference"))
  (`TextRenderComponent.K2_SetText` (`self.TextRender`) (`KismetTextLibrary.Conv_StringToText` "Processing"))
  (`KismetArrayLibrary.Array_Shuffle` _array)
  (`KismetSystemLibrary.Delay` 2.0)
  (`|SpawnActorFromClass` (`KismetArrayLibrary.Array_Random` _array) (`SceneComponent.K2_GetComponentToWorld` (`self.Ball Spawn Pos`)) "Undefined" "MultiplyWithRoot" null null)
  (set `self.ItemCount` (- (`self.ItemCount`) 3))
  (`self.UpdateCount`))

(fn `UserConstructionScript`)