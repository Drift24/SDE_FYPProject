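; Fire portal hazard actor with open, damage, close and self-destroy stages, driven by timelines and Niagara effects.
; Opening moves the base mesh, animates a dynamic material parameter, activates the portal effect, then swaps in the GC mesh.
; Damage triggers a separate burst effect.
; Closing animates Niagara parameters, plays an end effect, fades the material, spawns a master field below the GC mesh to break it, then destroys the actor.
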(event `openPortal`
  (`self.portalBegin`)
  (`KismetSystemLibrary.Delay` 0.3)
  (`self.matChange`)
  (bind (_direction _lerpfireopacity) (`Timeline|LerpFireOpacity`)
    (:`Update`
      (`MaterialInstanceDynamic.SetScalarParameterValue` (`self.DynamicScalarParam`) (`self.Parameter Name`) _lerpfireopacity))
    (:`Finished`
      (`KismetSystemLibrary.Delay` 0.2)
      (`ActorComponent.Activate` (`self.NS_Fire_PortalFX`) false)
      (`|ExecutionSequence`
        (:`then_0`
          (`KismetSystemLibrary.PrintString` "Portal Open" true true (struct :`G` 0.66 :`B` 1.0 :`A` 1.0) 5.0))
        (:`then_1`
          (`SceneComponent.SetVisibility` (`self.Fire_MainMesh`) false false))
        (:`then_2`
          (`SceneComponent.SetVisibility` (`self.GC_Fire_MainMesh`) true false))))))

(event `damagePortal`
  (`ActorComponent.Activate` (`self.NS_FirePortalDamage`) true)
  (`KismetSystemLibrary.PrintString` "Portal Damaged" true true (struct :`G` 0.66 :`B` 1.0 :`A` 1.0) 5.0))

(event `closePortal`
  (bind _ns_fire_portalfx (`self.NS_Fire_PortalFX`))
  (bind (_direction _opacitydynamicdensity _scaleashaura _scalemagicring_1 _scalemagicring_2 _scaleswirlin _scaleslushyring _opacitysparks) (`Timeline|lerp`)
    (:`Update`
      (`|ExecutionSequence`
        (:`then_0`
          (`NiagaraComponent.SetVariableFloat` _ns_fire_portalfx "opacityDynamicdensityRing" _opacitydynamicdensity))
        (:`then_1`
          (`NiagaraComponent.SetVariableFloat` _ns_fire_portalfx "scaleAshAura" _scaleashaura))
        (:`then_2`
          (`NiagaraComponent.SetVariableFloat` _ns_fire_portalfx "scaleMagicRing_1" _scalemagicring_1))
        (:`then_3`
          (`NiagaraComponent.SetVariableFloat` _ns_fire_portalfx "scaleMagicRing_2" _scalemagicring_2))
        (:`then_4`
          (`NiagaraComponent.SetVariableFloat` _ns_fire_portalfx "scaleSwirlIn" _scaleswirlin))
        (:`then_5`
          (`NiagaraComponent.SetVariableFloat` _ns_fire_portalfx "scaleSlushyRing" _scaleslushyring))
        (:`then_6`
          (`NiagaraComponent.SetVariableFloat` _ns_fire_portalfx "opacitySparks" _opacitysparks)
          (`ActorComponent.Deactivate` (`self.NS_Fire_PortalFX`))
          (`ActorComponent.Activate` (`self.NS_FirePortalEnd`) false)
          (`/Engine/EditorBlueprintResources/StandardMacros.DoOnce` false
            (:`Completed`
              (`KismetSystemLibrary.PrintString` "Portal Closed" true true (struct :`G` 0.66 :`B` 1.0 :`A` 1.0) 5.0)
              (`KismetSystemLibrary.Delay` 1.8)
              (bind (_direction_2 _lerpfadeaway) (`Timeline|LerpFadeAway` :!via `PlayFromStart`)
                (:`Update`
                  (`MaterialInstanceDynamic.SetScalarParameterValue` (`self.DynamicScalarParam`) (`self.Parameter Name`) _lerpfadeaway)
                  (`self.destroyPortalBase`)
                  (`KismetSystemLibrary.Delay` 6.0)
                  (`self.killMe`))))))))))

(event `killMe`
  (`self.K2_DestroyActor`)
  (`KismetSystemLibrary.PrintString` "Portal Killed" true true (struct :`G` 0.66 :`B` 1.0 :`A` 1.0) 5.0))

(event `self.ReceiveTick`
  (params (DeltaSeconds :type "Float (single-precision)")))

(event `matChange`
  (bind _fire_mainmesh (`self.Fire_MainMesh`))
  (bind _returnvalue (`KismetMaterialLibrary.CreateDynamicMaterialInstance` (`PrimitiveComponent.GetMaterial` _fire_mainmesh 1)))
  (bind _output_get (set `self.DynamicScalarParam` _returnvalue))
  (`PrimitiveComponent.SetMaterial` _fire_mainmesh 1 _output_get)
  (`PrimitiveComponent.SetMaterial` (`self.GC_Fire_MainMesh`) 1 _output_get))

(event `MoveUp`
  (bind _fire_mainmesh (`self.Fire_MainMesh`))
  (bind _returnvalue_location (`KismetMathLibrary.BreakTransform` (`SceneComponent.GetRelativeTransform` _fire_mainmesh)))
  ;[0.3125 0.3125 0.3125] Sean Seah Code cuz he is so hot and sexy and i love his tiddies his tits are always briked up and it is lowkey kidna hot and cute
  (`SceneComponent.K2_SetRelativeLocation` _fire_mainmesh (`KismetMathLibrary.VLerp` _returnvalue_location (0.0 0.0 0.0) (/ (`self.CurrentMoveTime`) (`self.TimeToReach`))) false true))

(event `portalBegin`
  (bind (_direction _portalstart) (`Timeline|portalStart`)
    (:`Update`
      (`SceneComponent.K2_SetRelativeLocation` (`self.Fire_MainMesh`) _portalstart false false))))

(fn `destroyPortalBase`
  (bind (_returnvalue_x _returnvalue_y _returnvalue_z) (`KismetMathLibrary.BreakVector` (`SceneComponent.K2_GetComponentLocation` (`self.GC_Fire_MainMesh`))))
  (`|SpawnActorFromClass` "/Game/FYP/FireHazard_1/Blueprint_Components/FS_Custom_MasterField.FS_Custom_MasterField_C" (`KismetMathLibrary.Conv_VectorToTransform` (`KismetMathLibrary.MakeVector` _returnvalue_x _returnvalue_y (- _returnvalue_z 100.0))) "Undefined" "MultiplyWithRoot" null null))

(fn `UserConstructionScript`)