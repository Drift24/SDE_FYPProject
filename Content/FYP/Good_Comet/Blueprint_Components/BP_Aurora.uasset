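; BP_Aurora is an aurora visual effect that other logic shows and hides through the openAurora and closeAurora events.
; Each event plays its own opacity timeline from the start, writing the animated value to the AuroraAppear vector parameter on the Aurora component's materials.
; Both timelines print a debug message when they finish.
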(event `openAurora`
  (bind (_direction _opacity) (`Timeline|lerpOpacity+` :!via `PlayFromStart`)
    (:`Update`
      (`MeshComponent.SetVectorParameterValueOnMaterials` (`self.Aurora`) (`self.Aurora Appear`) _opacity))
    (:`Finished`
      (`KismetSystemLibrary.PrintString` "Aurora Opened"))))

(event `closeAurora`
  (bind (_direction _opacity) (`Timeline|lerpOpacity-` :!via `PlayFromStart`)
    (:`Update`
      (`MeshComponent.SetVectorParameterValueOnMaterials` (`self.Aurora`) (`self.Aurora Appear`) _opacity))
    (:`Finished`
      (`KismetSystemLibrary.PrintString` "Aurora Closed"))))

(fn `UserConstructionScript`)